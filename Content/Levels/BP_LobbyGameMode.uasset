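; BP_LobbyGameMode is a lobby game mode that gives each joining player a spot and a shared camera view.
; On PostLogin, after a short delay, it uses the newest PlayerArray index to pick an actor tagged LobbySpot.
; It spawns an actor at that spot and switches the player's view target to the level's CameraActor.
; Without a valid spot, it only prints a debug string.
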(event `self.K2_PostLogin`
  (params (NewPlayer :type "PlayerController Object Reference"))
  (`KismetSystemLibrary.Delay` 0.2)
  (bind _output_get (set `self.PlayerIndex` (- (`KismetArrayLibrary.Array_Length` (`GameStateBase.PlayerArray` (`GameplayStatics.GetGameState`))) 1)))
  (bind _outactors (`GameplayStatics.GetAllActorsOfClassWithTag` "/Script/Engine.Actor" "LobbySpot"))
  (bind _output (`|GetArrayItem` _outactors _output_get))
  (`/Engine/EditorBlueprintResources/StandardMacros.IsValid` _output
    (:`Is Valid`
      (`|SpawnActorFromClass` "/Game/ThirdPerson/Models/BP_LobbyDummy.BP_LobbyDummy_C" (`self.GetTransform` _output) "Undefined" "MultiplyWithRoot" null null)
      (bind _returnvalue (`GameplayStatics.GetActorOfClass` "/Script/Engine.CameraActor"))
      (`PlayerController.SetViewTargetWithBlend` NewPlayer _returnvalue 0.0 "VTBlend_Linear" 0.0 false))
    (:`Is Not Valid`
      (`KismetSystemLibrary.PrintString` "Hello"))))

(fn `UserConstructionScript`)